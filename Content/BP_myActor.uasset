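; BP_myActor is an actor whose static mesh slides back and forth along relative X between roughly 0 and 100.
; While ISPLAY is true, Tick steps X위치 one unit per frame, independent of delta time, and flips Ismoveright at either limit.
; BeginPlay only prints a debug string.
; Unconnected leftovers hold a delayed step-move sequence, a self-name print and stray math and comparison nodes.
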(event EventBeginPlay
  ;[1 1 1] 실행한다
  (Development|PrintString "beginplay"))

(event EventTick
  (params (DeltaSeconds :type Float%20%28single-precision%29))
  ;[1 1 1] 반복되는 이벤트가 발생한다
  (if (Variables|Default|GetISPLAY)
    ;[1 1 1] 만약에
    (if (Variables|Default|Getismoveright)
      ;[1 1 1] 움직인다
      ;;[1 1 1] x 방향으로 한 번 움직인다
      ;;;[1 1 1] 위치를 설정한다
      (bind _output_get (Variables|Default|SetX위치 (+ (Variables|Default|GetX위치) 1.0)))
      (Transformation|SetRelativeLocation (Variables|Default|GetStaticMesh) (Math|Vector|MakeVector _output_get 0.0 0.0) false false)
      ;;[1 1 1] 만약 (사실)이면
      (if (> (Variables|Default|GetX위치) 1e+02)
        ;;[1 1 1] (Set)움직일지 결정한다
        (Variables|Default|Setismoveright false))
      (else
        ;;[1 1 1] x 반대 방향으로 한 번 움직인다
        (bind _output_get_2 (Variables|Default|SetX위치 (+ (Variables|Default|GetX위치) -1.0)))
        (Transformation|SetRelativeLocation (Variables|Default|GetStaticMesh) (Math|Vector|MakeVector _output_get_2 0.0 0.0) false false)
        ;;[1 1 1] 만약 (사실)이면
        (if (< (Variables|Default|GetX위치) 0.0)
          ;;[1 1 1] 움직일지 결정한다
          (Variables|Default|Setismoveright true))))))

(fn ConstructionScript)